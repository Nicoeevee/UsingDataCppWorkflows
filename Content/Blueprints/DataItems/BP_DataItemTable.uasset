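; Item actor configured from a data table, showing a details widget while the player is near it.
; Unless RunCode is set, the construction script looks up the ItemType row, fills GenericItemInfo, sets the mesh and copies rotation curve and duration.
; Sphere overlap by the player creates or reuses WBP_WeaponData, and end overlap removes it.
; BeginPlay also exports the item table to TestFile.csv in the project content directory.
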(event `self.ReceiveBeginPlay`
  (`DataLibrary.SaveTable` (`KismetSystemLibrary.GetProjectContentDirectory`) "TestFile.csv" (`self.ItemDataTable`)))

(event `self.SphereCollider.OnComponentBeginOverlap`
  (params (OverlappedComponent :type "PrimitiveComponent Object Reference") (OtherActor :type "Actor Object Reference") (OtherComp :type "PrimitiveComponent Object Reference") (OtherBodyIndex :type Integer) (bFromSweep :type Boolean) (SweepResult :type "HitResult Structure (by ref)"))
  (if (== OtherActor (`GameplayStatics.GetPlayerPawn` 0))
    (`/Engine/EditorBlueprintResources/StandardMacros.IsValid` (`self.DetailsWidget`)
      (:`Is Valid`
        (`UserWidget.AddToViewport` (`self.DetailsWidget`) 0))
      (:`Is Not Valid`
        (bind _returnvalue (`|CreateWidget` "/Game/Blueprints/Widget/WBP_WeaponData.WBP_WeaponData_C"))
        (bind _output_get (set `self.DetailsWidget` _returnvalue))
        (`UserWidget.AddToViewport` _output_get 0)
        (`/Game/Blueprints/Widget/WBP_WeaponData.SetItemDetails` (`self.DetailsWidget`) (`self.GenericItemInfo`))))))

(event `self.SphereCollider.OnComponentEndOverlap`
  (params (OverlappedComponent :type "PrimitiveComponent Object Reference") (OtherActor :type "Actor Object Reference") (OtherComp :type "PrimitiveComponent Object Reference") (OtherBodyIndex :type Integer))
  (if (== OtherActor (`GameplayStatics.GetPlayerPawn` 0))
    (`/Engine/EditorBlueprintResources/StandardMacros.IsValid` (`self.DetailsWidget`)
      (:`Is Valid`
        (`Widget.RemoveFromParent` (`self.DetailsWidget`))))))

(fn `UserConstructionScript`
  (bind ((`Mesh` _mesh) (`CurveFloat` _curvefloat) (`RotationDuration` _rotationduration)) (break `GenericItemInfo` (`self.GenericItemInfo`)))
  (if (not (`self.bRunCode`))
    (bind _returnvalue (`|GetDataTableRow` (`self.ItemDataTable`) (`KismetStringLibrary.Conv_StringToName` (`|GetEnumeratorNameAsString` (`self.ItemType`))))
      (:`then`
        (bind (_itemtype _itemname _itemcost _iteminfo _mesh_2 _itemimage _curvefloat_2 _rotationduration_2) (break `ItemInformationTable` _returnvalue))
        (set `self.GenericItemInfo` (make `GenericItemInfo` _itemtype _itemname _itemcost _iteminfo _mesh_2 _itemimage _curvefloat_2 _rotationduration_2))
        (`StaticMeshComponent.SetStaticMesh` (`self.Mesh`) _mesh)
        (set `self.mFloatCurve` _curvefloat)
        (set `self.mRotationDuration` _rotationduration)))))